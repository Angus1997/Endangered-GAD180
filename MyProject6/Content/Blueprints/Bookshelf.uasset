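; Interactive bookshelf Blueprint that lets a player use E while inside its collider, with overlap begin and end toggling input.
; Each press shows an event widget and alternates the Rotation timeline forward or reverse; releasing adds a second interface widget.
; The timeline's Finished output, rather than Update, sets both bookshelves' pitch and disables their collision, which is never re-enabled.
; An author note flags a collision issue.
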(event `self.Collider.OnComponentBeginOverlap`
  (params (OverlappedComponent :type "PrimitiveComponent Object Reference") (OtherActor :type "Actor Object Reference") (OtherComp :type "PrimitiveComponent Object Reference") (OtherBodyIndex :type Integer) (bFromSweep :type Boolean) (SweepResult :type "HitResult Structure (by ref)"))
  ;[1 1 1] Door Input
  (`self.EnableInput` (`GameplayStatics.GetPlayerController` 0)))

(event `Key|E`
  (params (Key :type "Key Structure"))
  (bind _bookshelf2 (`self.Bookshelf2`))
  ;[1 1 1] Stands Bookshelves Up but has issue with collision
  (:`Pressed`
    (bind _returnvalue (`|CreateWidget` "/Game/UI/Widgets/BookshelfEventHappen.BookshelfEventHappen_C"))
    (`UserWidget.AddToViewport` _returnvalue 0)
    (`/Engine/EditorBlueprintResources/StandardMacros.FlipFlop`
      (:`A`
        (bind (_direction _newtrack_0) (`Timeline|Rotation` :!label _label)
          (:`Finished`
            (`SceneComponent.K2_SetRelativeRotation` _bookshelf2 (`KismetMathLibrary.MakeRotator` 0.0 _newtrack_0) false false)
            (`SceneComponent.K2_SetRelativeRotation` (`self.Bookshelf`) (`KismetMathLibrary.MakeRotator` 0.0 _newtrack_0) false false)
            (`PrimitiveComponent.SetCollisionEnabled` _bookshelf2 "NoCollision")
            (`PrimitiveComponent.SetCollisionEnabled` (`self.Bookshelf`) "NoCollision"))))
      (:`B`
        (goto _label :!via `Reverse`))))
  (:`Released`
    (bind _returnvalue_2 (`|CreateWidget` "/Game/UI/Widgets/ButtonForTurningOffInterface.ButtonForTurningOffInterface_C"))
    (`UserWidget.AddToViewport` _returnvalue_2 0)))

(event `self.Collider.OnComponentEndOverlap`
  (params (OverlappedComponent :type "PrimitiveComponent Object Reference") (OtherActor :type "Actor Object Reference") (OtherComp :type "PrimitiveComponent Object Reference") (OtherBodyIndex :type Integer))
  ;[1 1 1] Door Input
  (`self.DisableInput` (`GameplayStatics.GetPlayerController` 0)))

(fn `UserConstructionScript`)