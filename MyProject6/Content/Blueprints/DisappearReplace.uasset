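; Interactable level actor that fixes a busted floor and chandelier event by toggling their visibility.
; Player overlap with PlayerDetect registers it as the TopDownCharacter's InteractObject, swaps the chandelier to a highlight material and enables input; leaving reverts all three.
; Interacting sets Fix, shows UI widgets, plays a creak, toggles floor, chandelier and FloorMover visibility, removes floor and chandelier collision, then calls CallActionCompleted.
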(event `self.PlayerDetect.OnComponentBeginOverlap`
  (params (OverlappedComponent :type "PrimitiveComponent Object Reference") (OtherActor :type "Actor Object Reference") (OtherComp :type "PrimitiveComponent Object Reference") (OtherBodyIndex :type Integer) (bFromSweep :type Boolean) (SweepResult :type "HitResult Structure (by ref)"))
  (bind _returnvalue (`GameplayStatics.GetPlayerCharacter` 0))
  ;[1 1 1] Controls Visibility of Broken Floor and Chandelier and also highlights interactivity of event
  (if (== OtherActor _returnvalue)
    (bind _astop_down_character (cast `/Game/TopDownBP/Blueprints/TopDownCharacter` _returnvalue))
    (set `/Game/TopDownBP/Blueprints/TopDownCharacter.Interact Object` self _astop_down_character)
    (`PrimitiveComponent.SetMaterial` (`self.Chandlier`) 0 "/Game/Blueprints/M_DisappearReplace.M_DisappearReplace")
    (`PrimitiveComponent.SetMaterial` (`self.Chandlier`) 1 "/Game/Blueprints/M_DisappearReplace.M_DisappearReplace")
    (`self.EnableInput` (`GameplayStatics.GetPlayerController` 0))))

(event `interact`
  (bind _bustedfloor (`self.BustedFloor`))
  ;[1 1 1] Controls Visibility of Broken Floor and Chandelier and also highlights interactivity of event
  (set `self.Fix` true)
  (bind _astop_down_character (cast `/Game/TopDownBP/Blueprints/TopDownCharacter` (`GameplayStatics.GetPlayerCharacter` 0)))
  (`/Game/TopDownBP/Blueprints/TopDownCharacter.Activate Widget` _astop_down_character "/Game/UI/Widgets/ButtonForTurningOffInterface.ButtonForTurningOffInterface_C")
  (bind _returnvalue (`|CreateWidget` "/Game/UI/Widgets/EventHappen.EventHappen_C"))
  (`GameplayStatics.PlaySoundAtLocation` "/Game/Unsettling_Squeakes_and_Creaks/wavs/Wooden-Door_Creak_46.Wooden-Door_Creak_46" (`SceneComponent.K2_GetComponentLocation` (`self.BustedFloor`)) (struct) 1.0 1.0 0.0 null null null)
  (`UserWidget.AddToViewport` _returnvalue 0)
  (`SceneComponent.ToggleVisibility` _bustedfloor false)
  (`SceneComponent.ToggleVisibility` (`self.Chandlier`) false)
  (`SceneComponent.ToggleVisibility` (`self.Floor Mover`) false)
  (`PrimitiveComponent.SetCollisionEnabled` _bustedfloor "NoCollision")
  (`PrimitiveComponent.SetCollisionEnabled` (`self.Chandlier`) "NoCollision")
  (`self.ActionCompleted`))

(event `self.PlayerDetect.OnComponentEndOverlap`
  (params (OverlappedComponent :type "PrimitiveComponent Object Reference") (OtherActor :type "Actor Object Reference") (OtherComp :type "PrimitiveComponent Object Reference") (OtherBodyIndex :type Integer))
  (bind _returnvalue (`GameplayStatics.GetPlayerCharacter` 0))
  ;[1 1 1] Controls Visibility of Broken Floor and Chandelier and also highlights interactivity of event
  (if (== OtherActor _returnvalue)
    (bind _astop_down_character (cast `/Game/TopDownBP/Blueprints/TopDownCharacter` _returnvalue))
    (set `/Game/TopDownBP/Blueprints/TopDownCharacter.Interact Object` null _astop_down_character)
    (`PrimitiveComponent.SetMaterial` (`self.Chandlier`) 0 "/Game/TopDownInteriors/Shared/Materials/M_Addons1_Alpha.M_Addons1_Alpha")
    (`PrimitiveComponent.SetMaterial` (`self.Chandlier`) 1 "/Game/TopDownInteriors/Shared/Materials/M_Addons1.M_Addons1")
    (`self.DisableInput` (`GameplayStatics.GetPlayerController` 0))))

(fn `UserConstructionScript`)