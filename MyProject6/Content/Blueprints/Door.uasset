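; Interactable door that swings open once three puzzle actions are completed.
; On BeginPlay it binds completion events on the DisappearReplace, Bookshelf and Chairs actors, each incrementing ActionCount.
; A box overlap registers the door as the player character's InteractObject, swaps in a highlight material and enables input, reverting on exit.
; When the count is met, interact sets Fix and plays a timeline that drives the door's yaw.
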(event `interact`
  ;[1 1 1] opens door
  (if (>= (`self.ActionCount`) 3)
    (set `self.Fix` true)
    (cast `/Game/TopDownBP/Blueprints/TopDownCharacter` (`GameplayStatics.GetPlayerCharacter` 0))
    (bind (_direction _standchair) (`Timeline|Timeline_0` :`NewTime` 2.0)
      (:`Update`
        _)
      (:`Finished`
        _))
    (`SceneComponent.K2_SetRelativeRotation` (`self.Door`) (`KismetMathLibrary.MakeRotator` 0.0 0.0 _standchair) false false)))

(event `self.Box.OnComponentBeginOverlap`
  (params (OverlappedComponent :type "PrimitiveComponent Object Reference") (OtherActor :type "Actor Object Reference") (OtherComp :type "PrimitiveComponent Object Reference") (OtherBodyIndex :type Integer) (bFromSweep :type Boolean) (SweepResult :type "HitResult Structure (by ref)"))
  (bind _returnvalue (`GameplayStatics.GetPlayerCharacter` 0))
  ;[1 1 1] Detects player and changes material to highlight
  (if (== OtherActor _returnvalue)
    (bind _astop_down_character (cast `/Game/TopDownBP/Blueprints/TopDownCharacter` _returnvalue))
    (set `/Game/TopDownBP/Blueprints/TopDownCharacter.Interact Object` self _astop_down_character)
    (`PrimitiveComponent.SetMaterial` (`self.Door`) 0 "/Game/Blueprints/M_DisappearReplace.M_DisappearReplace")
    (`self.EnableInput` (`GameplayStatics.GetPlayerController` 0))))

(event `self.Box.OnComponentEndOverlap`
  (params (OverlappedComponent :type "PrimitiveComponent Object Reference") (OtherActor :type "Actor Object Reference") (OtherComp :type "PrimitiveComponent Object Reference") (OtherBodyIndex :type Integer))
  (bind _returnvalue (`GameplayStatics.GetPlayerCharacter` 0))
  ;[1 1 1] Detects player and changes material to highlight
  (if (== OtherActor _returnvalue)
    (bind _astop_down_character (cast `/Game/TopDownBP/Blueprints/TopDownCharacter` _returnvalue))
    (set `/Game/TopDownBP/Blueprints/TopDownCharacter.Interact Object` null _astop_down_character)
    (`PrimitiveComponent.SetMaterial` (`self.Door`) 0 "/Game/TopDownInteriors/Shared/Materials/M_Atlas1.M_Atlas1")
    (`self.DisableInput` (`GameplayStatics.GetPlayerController` 0))))

(event `self.ReceiveBeginPlay`
  (bind _returnvalue (`GameplayStatics.GetActorOfClass` "/Game/Blueprints/DisappearReplace.DisappearReplace_C"))
  (add `/Game/Blueprints/DisappearReplace.ActionCompleted` _returnvalue (delegate `Action Completed`))
  (bind _returnvalue_2 (`GameplayStatics.GetActorOfClass` "/Game/Blueprints/Bookshelf.Bookshelf_C"))
  (add `/Game/Blueprints/Bookshelf.ActionCompleted` _returnvalue_2 (delegate `Action Completed`))
  (bind _returnvalue_3 (`GameplayStatics.GetActorOfClass` "/Game/TopDownInteriors/Chairs.Chairs_C"))
  (add `/Game/TopDownInteriors/Chairs.ActionCompleted` _returnvalue_3 (delegate `Action Completed`)))

(event `Action Completed`
  (`/Engine/EditorBlueprintResources/StandardMacros.IncrementInt` (`self.ActionCount`)
    (:`  `
      (`KismetSystemLibrary.PrintString` "help"))))

(fn `UserConstructionScript`)