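; CreepyEvent is a one-shot triggered scare that briefly shows a moving Steam component when the player walks into its detection volume.
; Steam starts hidden, and an overlap on Detectplayer checks that the player character's capsule is inside before revealing it.
; A timed MoveComponentTo slides Steam along its relative X axis, then it is hidden again and the trigger's collision is disabled.
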(event `self.ReceiveBeginPlay`
  (`SceneComponent.SetVisibility` (`self.Steam`) false false))

(event `self.detectplayer.OnComponentBeginOverlap`
  (params (OverlappedComponent :type "PrimitiveComponent Object Reference") (OtherActor :type "Actor Object Reference") (OtherComp :type "PrimitiveComponent Object Reference") (OtherBodyIndex :type Integer) (bFromSweep :type Boolean) (SweepResult :type "HitResult Structure (by ref)"))
  (if (`PrimitiveComponent.IsOverlappingComponent` (`Character.CapsuleComponent` (`GameplayStatics.GetPlayerCharacter` 0)) (`self.detectplayer`))
    (`SceneComponent.SetVisibility` (`self.Steam`) true false)
    (`KismetSystemLibrary.MoveComponentTo` (`self.Steam`) (-500.0 0.0 0.0) (struct) false false 1.5)
    (`SceneComponent.SetVisibility` (`self.Steam`) false false)
    (`PrimitiveComponent.SetCollisionEnabled` (`self.detectplayer`) "NoCollision")))

(fn `UserConstructionScript`)